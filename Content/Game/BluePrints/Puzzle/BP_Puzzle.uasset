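; BP_Puzzle is a three-key rotation puzzle that moves a linked platform once every key matches its code.
; Interact yaws the given key component left or right by a set step and prints its rotation.
; CheckCode identifies the key, compares its relative yaw to the target within a tolerance, and stores the result per key.
; When no stored result is false, it calls MovePlatform on the Platform.
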(event `/Game/ThirdPersonCharacter/Interfaces/BP_GameplayInterface.Interact`
  (params (Component :type "PrimitiveComponent Object Reference") (`Rotate Left` :type Boolean))
  (`self.Rotate` `Rotate Left` Component))

(fn `Check Code`
  (params (Component :type "PrimitiveComponent Object Reference"))
  (locals (SelectedMesh :type Integer) (LocalFail :type Boolean))
  (bind (_relativerotation_roll _relativerotation_pitch _relativerotation_yaw) (`KismetMathLibrary.BreakRotator` (`SceneComponent.RelativeRotation` Component)))
  (if (== Component (`self.FirstKey`))
    (set `local.SelectedMesh` 0)
    (`KismetArrayLibrary.Array_Set` (`self.CorrectCode`) (`local.SelectedMesh`) (`KismetMathLibrary.NearlyEqual_FloatFloat` (`|GetArrayItem` (`self.Code`) (`local.SelectedMesh`)) _relativerotation_yaw 35.0) :!label _label)
    (for _array_element (`self.CorrectCode`)
      (if (not _array_element)
        (set `local.LocalFail` true)))
    (if (not (`local.LocalFail`))
      (`/Game/Game/BluePrints/Puzzle/BP_Platform.MovePlatform` (`self.Platform`)))
    (elif (== Component (`self.SecondKey`))
      (set `local.SelectedMesh` 1)
      (goto _label)
      (elif (== Component (`self.ThirdKey`))
        (set `local.SelectedMesh` 2)
        (goto _label)))))

(fn `Rotate`
  (params (`Rotate Left` :type Boolean) (Component :type "PrimitiveComponent Object Reference"))
  (if `Rotate Left`
    (`SceneComponent.K2_AddRelativeRotation` Component (`KismetMathLibrary.MakeRotator` 0.0 0.0 (* (`self.Rotation Value`) -1.0)) false false)
    (else
      (`SceneComponent.K2_AddRelativeRotation` Component (`KismetMathLibrary.MakeRotator` 0.0 0.0 (`self.Rotation Value`)) false false)))
  (`KismetSystemLibrary.PrintString` (`KismetStringLibrary.Conv_RotatorToString` (`SceneComponent.RelativeRotation` Component)))
  (`self.Check Code` Component))

(fn `UserConstructionScript`)